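; Base character Blueprint for the Gameplay Ability System, providing health regen, dash and melee abilities plus death, knockback and stun handling.
; BeginPlay grants the configured abilities, and events activate them by class.
; Sword and capsule overlaps send melee and dash damage gameplay events against hostile characters, with an exclusion list preventing repeat dash hits.
; Push temporarily zeroes ground friction around an impulse, and death plays a montage before destroying the actor.
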(event `self.ReceiveBeginPlay`
  (`parent.ReceiveBeginPlay`)
  (`self.EvCpp_AquireAbilitys` (`self.AbilityToAquires`)))

(event `EvTryHealthRegen`
  (`AbilitySystemComponent.TryActivateAbilityByClass` (`self.AbilitySystemComp`) "/Game/AbilitySystem/Core/Blueprints/GameplayAbilities/HealthRegen/GA_HealthRegen.GA_HealthRegen_C" true))

(event `EvTryDashAbility`
  (`AbilitySystemComponent.TryActivateAbilityByClass` (`self.AbilitySystemComp`) "/Game/AbilitySystem/Core/Blueprints/GameplayAbilities/Dash/GA_Dash.GA_Dash_C" true))

(event `EvMeleeAttack`
  (`AbilitySystemComponent.TryActivateAbilityByClass` (`self.AbilitySystemComp`) "/Game/AbilitySystem/Core/Blueprints/GameplayAbilities/Melee/GA_Melee.GA_Melee_C" true))

(event `self.SwordColliedr.OnComponentBeginOverlap`
  (params (OverlappedComponent :type "PrimitiveComponent Object Reference") (OtherActor :type "Actor Object Reference") (OtherComp :type "PrimitiveComponent Object Reference") (OtherBodyIndex :type Integer) (bFromSweep :type Boolean) (SweepResult :type "HitResult Structure (by ref)"))
  (if (!= self OtherActor)
    (bind _asbp_character_base (cast `/Game/AbilitySystem/Core/Blueprints/Characters/Bp_CharacterBase` OtherActor))
    (bind _returnvalue (`self.FCppIsOtherHosttile` _asbp_character_base self))
    (if _returnvalue
      (`AbilitySystemBlueprintLibrary.SendGameplayEventToActor` self (struct :`TagName` "skill.melee.dealDamage") (make `GameplayEventData` (struct) null OtherActor)))))

(event `self.BP_Die`
  (bind _returnvalue (`self.PlayAnimMontage` "/Game/AbilitySystem/Animations/Shinbi/AM_Death_A_Shinbi.AM_Death_A_Shinbi"))
  (`KismetSystemLibrary.Delay` _returnvalue)
  (`self.K2_DestroyActor`))

(event `EvSetCollisionToPawn`
  (params (NewResponse :type "ECollisionResponse Enum" :default "ECR_Ignore"))
  (`PrimitiveComponent.SetCollisionResponseToChannel` (`self.CapsuleComponent`) "ECC_Pawn" NewResponse))

(event `self.CapsuleComponent.OnComponentBeginOverlap`
  (params (OverlappedComponent :type "PrimitiveComponent Object Reference") (OtherActor :type "Actor Object Reference") (OtherComp :type "PrimitiveComponent Object Reference") (OtherBodyIndex :type Integer) (bFromSweep :type Boolean) (SweepResult :type "HitResult Structure (by ref)"))
  (bind _asbp_character_base (cast `/Game/AbilitySystem/Core/Blueprints/Characters/Bp_CharacterBase` OtherActor))
  (bind _returnvalue (`self.FCppIsOtherHosttile` _asbp_character_base self))
  (if _returnvalue
    (if (not (`KismetArrayLibrary.Array_Contains` (`self.OverlapExclude`) _asbp_character_base))
      (`KismetArrayLibrary.Array_AddUnique` (`self.OverlapExclude`) _asbp_character_base)
      (`AbilitySystemBlueprintLibrary.SendGameplayEventToActor` self (struct :`TagName` "skill.dash.dealDamage") (make `GameplayEventData` (struct) self OtherActor)))))

(event `EvPushCharacter`
  (params (ImpulseDirection :type "Vector Structure") (PushStrength :type "Float (double-precision)") (StunDuration :type "Float (double-precision)"))
  (bind _charactermovement (`self.CharacterMovement`))
  (set `self.DefaultGroundFriction` (`CharacterMovementComponent.GroundFriction` _charactermovement))
  (set `CharacterMovementComponent.GroundFriction` 0.0 _charactermovement)
  (`CharacterMovementComponent.AddImpulse` (`self.CharacterMovement`) (* ImpulseDirection PushStrength) true)
  (if (> StunDuration 0.0)
    (`self.EvCpp_HitStun` StunDuration))
  (`KismetSystemLibrary.Delay` 0.3)
  (set `CharacterMovementComponent.GroundFriction` (`self.DefaultGroundFriction`) (`self.CharacterMovement`)))

(event `EvClearDash`
  (`KismetArrayLibrary.Array_Clear` (`self.OverlapExclude`)))

(fn `UserConstructionScript`)