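; Base enemy character Blueprint that drives a health bar widget on top of its parent class's behavior.
; BeginPlay casts the health bar component's user widget to WBP_HealthBar and caches the reference.
; Health change events forward the percentage to that widget, and the death event calls the parent logic, then hides the bar.
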(event `self.ReceiveBeginPlay`
  (`parent.ReceiveBeginPlay`)
  (bind _aswbp_health_bar (cast `/Game/AbilitySystem/Core/UI/Childs/WBP_HealthBar` (`WidgetComponent.GetUserWidgetObject` (`self.WBP_HealthBar`))))
  (set `self.WBPHealthBar` _aswbp_health_bar))

(fn `UserConstructionScript`
  (`parent.UserConstructionScript`))