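; Base Gameplay Ability Blueprint that provides shared helpers for character abilities: knockback, owner lookup and UI cooldown feedback.
; The push event sends a target character away from the ability owner along a normalized direction, passing strength and stun duration to the character's own push event.
; A lookup returns the owning character and player controller, which the cooldown function uses to start cooldowns on primary UI slots matching this ability's class.
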(event `EvPushCharacter`
  (params (actor :type "Actor Object Reference") (PushStrength :type "Float (double-precision)") (StunDuration :type "Float (double-precision)"))
  (bind _asbp_character_base (cast `/Game/AbilitySystem/Core/Blueprints/Characters/Bp_CharacterBase` actor))
  (`/Game/AbilitySystem/Core/Blueprints/Characters/Bp_CharacterBase.EvPushCharacter` _asbp_character_base (`KismetMathLibrary.Normal` (- (`Actor.K2_GetActorLocation` _asbp_character_base) (`Actor.K2_GetActorLocation` (`self.GetOwningActorFromActorInfo`)))) PushStrength StunDuration))

(fn `FDoUICooldown`
  (bind (_character _controller) (`self.FGet Player Info`))
  (`/Engine/EditorBlueprintResources/StandardMacros.IsValid` _controller
    (:`Is Valid`
      (for _array_element (`/Game/AbilitySystem/Core/UI/WBP_PrimaryUI.Slots` (`/Game/AbilitySystem/Core/Blueprints/Characters/Player/BP_PlayerControllerBase.WBP_PrimaryUI` _controller))
        (bind _returnvalue (`self.GetAbilityInfo`))
        (if (== (`.AbilityClass` (break `GameplayAbilityInfo` _returnvalue)) (`.AbilityClass` (break `GameplayAbilityInfo` (`/Game/AbilitySystem/Core/UI/Childs/WBP_AbilitySlot.AbilityInfo` _array_element))))
          (`/Game/AbilitySystem/Core/UI/Childs/WBP_AbilitySlot.EvStartCooldown` _array_element))))))

(fn `FGet Player Info`
  (returns (Character :type "/Game/AbilitySystem/Core/Blueprints/Characters/Bp_CharacterBase Object Reference") (Controller :type "/Game/AbilitySystem/Core/Blueprints/Characters/Player/BP_PlayerControllerBase Object Reference"))
  (bind _asbp_character_base (cast `/Game/AbilitySystem/Core/Blueprints/Characters/Bp_CharacterBase` (`self.GetOwningActorFromActorInfo`)))
  (bind _asbp_player_controller_base (cast `/Game/AbilitySystem/Core/Blueprints/Characters/Player/BP_PlayerControllerBase` (`Pawn.GetController` _asbp_character_base))
    (:`then`
      _)
    (:`CastFailed`
      _))
  (return _asbp_character_base _asbp_player_controller_base))