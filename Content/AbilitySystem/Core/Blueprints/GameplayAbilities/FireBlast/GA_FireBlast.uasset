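; Fire Blast gameplay ability that pulls nearby characters toward the caster, then damages and blasts them away.
; It commits, starts the UI cooldown and plays a montage whose gameplay events time both phases.
; The pull event gathers targets instantly around the caster and caches their data for the push event.
; Both phases stun, but every push reuses one direction from the last pulled character instead of each target's own.
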(event `self.K2_ActivateAbility`
  (bind _targetdatahandle (`self.TargetDataHandle`))
  (`self.K2_CommitAbility`)
  (`self.FDoUICooldown`)
  (`AbilityTask_PlayMontageAndWait.CreatePlayMontageAndWaitProxy` "None" "/Game/AbilitySystem/Animations/Shinbi/AM_FireBlast_Shinbi.AM_FireBlast_Shinbi"
    (:`then`
      (`AbilityTask_WaitGameplayEvent.WaitGameplayEvent` (struct :`TagName` "skill.fireBlast.pull") null
        (:`EventReceived`
          (bind (_asynctaskproxy _data) (`AbilityTask_WaitTargetData.WaitTargetData` "None" "Instant" "/Script/AbilitySystem2.CppTargetActorGetAround" 1000.0 (struct) (struct) null)
            (:`then`
              (`AbilityTask_WaitGameplayEvent.WaitGameplayEvent` (struct :`TagName` "skill.fireBlast.push") null
                (:`EventReceived`
                  (`self.BP_ApplyGameplayEffectToTarget` _targetdatahandle "/Game/AbilitySystem/Core/Blueprints/GameplayAbilities/FireBlast/attr/GE_FireBlast_Damage.GE_FireBlast_Damage_C")
                  (for _array_element (`AbilitySystemBlueprintLibrary.GetActorsFromTargetData` _targetdatahandle)
                    (bind _asbp_character_base (cast `/Game/AbilitySystem/Core/Blueprints/Characters/Bp_CharacterBase` _array_element))
                    (bind _returnvalue (`KismetMathLibrary.Normal` (- (`Actor.K2_GetActorLocation` (`self.GetOwningActorFromActorInfo`)) (`Actor.K2_GetActorLocation` (stale _asbp_character_base_2)))))
                    (`/Game/AbilitySystem/Core/Blueprints/Characters/Bp_CharacterBase.EvPushCharacter` _asbp_character_base (* _returnvalue -1.0) 2000.0 2.0 null)))))
            (:`ValidData`
              (set `self.TargetDataHandle` _data)
              (for _array_element_2 (`AbilitySystemBlueprintLibrary.GetActorsFromTargetData` _data)
                (bind _asbp_character_base_2 (cast `/Game/AbilitySystem/Core/Blueprints/Characters/Bp_CharacterBase` _array_element_2))
                (`/Game/AbilitySystem/Core/Blueprints/Characters/Bp_CharacterBase.EvPushCharacter` _asbp_character_base_2 _returnvalue 1000.0 3.0 null)))))))
    (:`OnCompleted`
      (`self.K2_EndAbility` :!label _label))
    (:`OnBlendOut`
      (goto _label))
    (:`OnInterrupted`
      (goto _label))
    (:`OnCancelled`
      (goto _label))))