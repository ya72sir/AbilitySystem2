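; Gameplay ability for a Ground Blast: a player-targeted area attack that damages and launches characters.
; It plays a targeting montage, waits out its length, then awaits user-confirmed data from a ground-select target actor.
; On confirm, it plays the cast montage, spawns the blast at the last target data point, applies the damage effect, and pushes hit characters upward with a stun.
; EndAbility is called only on cancel.
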(event `self.K2_ActivateAbility`
  (`AbilityTask_PlayMontageAndWait.CreatePlayMontageAndWaitProxy` "None" "/Game/AbilitySystem/Animations/Shinbi/AM_GroundBlast_Targeting.AM_GroundBlast_Targeting"
    (:`then`
      (`KismetSystemLibrary.Delay` (`AnimSequenceBase.SequenceLength` (`self.GetCurrentMontage`)))
      (bind (_asynctaskproxy _data) (`AbilityTask_WaitTargetData.WaitTargetData` "None" "UserConfirmed" "/Game/AbilitySystem/Core/Blueprints/GameplayAbilities/GroundBlast/BP_GATargetActorGroundSelect.BP_GATargetActorGroundSelect_C" 200.0 (struct) (struct) null)
        (:`ValidData`
          (`AbilityTask_PlayMontageAndWait.CreatePlayMontageAndWaitProxy` "None" "/Game/AbilitySystem/Animations/Shinbi/AM_Shinbi_GroundBlast_Cast.AM_Shinbi_GroundBlast_Cast"
            (:`then`
              (`GameplayStatics.SpawnEmitterAtLocation` "/Game/AbilitySystem/Library/ParticlesSystem/PS_GroundBlast.PS_GroundBlast" (`AbilitySystemBlueprintLibrary.GetTargetDataEndPoint` _data (- (`AbilitySystemBlueprintLibrary.GetDataCountFromTargetData` _data) 1)))
              (`self.BP_ApplyGameplayEffectToTarget` _data "/Game/AbilitySystem/Core/Blueprints/GameplayAbilities/GroundBlast/Attr/GE_GroundBlast_Damage.GE_GroundBlast_Damage_C")
              (for _array_element (`AbilitySystemBlueprintLibrary.GetActorsFromTargetData` _data)
                (bind _asbp_character_base (cast `/Game/AbilitySystem/Core/Blueprints/Characters/Bp_CharacterBase` _array_element))
                (`/Game/AbilitySystem/Core/Blueprints/Characters/Bp_CharacterBase.EvPushCharacter` _asbp_character_base (0.0 0.0 1.0) 500.0 2.0)))))
        (:`Cancelled`
          (`self.K2_EndAbility`))))))