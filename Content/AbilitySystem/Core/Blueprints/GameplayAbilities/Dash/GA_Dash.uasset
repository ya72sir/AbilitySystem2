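; GA_Dash is a Gameplay Ability that dashes the owning character forward, damaging, pushing and stunning targets it hits.
; It zeroes ground friction, applies a velocity-change impulse and sets pawn collision to overlap while the dash montage plays.
; A dealDamage gameplay event supplies each target for the damage effect and push.
; When the montage completes, blends out or is interrupted or cancelled, friction and collision are restored and the ability ends.
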(event `self.K2_ActivateAbility`
  (`self.K2_CommitAbility`)
  (`self.FDoUICooldown`)
  (bind _ascharacter (cast `Character` (`self.GetOwningActorFromActorInfo`))
    (:`then`
      (bind _charactermovement (`Character.CharacterMovement` _ascharacter))
      (set `self.OriginalGroundFriction` (`CharacterMovementComponent.GroundFriction` _charactermovement))
      (set `CharacterMovementComponent.GroundFriction` 0.0 _charactermovement)
      (`CharacterMovementComponent.AddImpulse` _charactermovement (* (`Actor.GetActorForwardVector` _ascharacter) 2000.0) true)
      (bind _character (`self.FGet Player Info`))
      (`/Game/AbilitySystem/Core/Blueprints/Characters/Bp_CharacterBase.EvSetCollisionToPawn` _character "ECR_Overlap")
      (`AbilityTask_PlayMontageAndWait.CreatePlayMontageAndWaitProxy` "None" "/Game/AbilitySystem/Animations/Shinbi/AM_Dash.AM_Dash"
        (:`then`
          (bind (_asynctaskproxy _payload) (`AbilityTask_WaitGameplayEvent.WaitGameplayEvent` (struct :`TagName` "skill.dash.dealDamage") null)
            (:`EventReceived`
              (bind (_eventtag _instigator _target) (break `GameplayEventData` _payload))
              (`self.BP_ApplyGameplayEffectToTarget` (`AbilitySystemBlueprintLibrary.AbilityTargetDataFromActor` _target) "/Game/AbilitySystem/Core/Blueprints/GameplayAbilities/Dash/Attr/GE_Dash_Damage.GE_Dash_Damage_C")
              (`self.EvPushCharacter` _target 4000.0 5.0))))
        (:`OnCompleted`
          (set `CharacterMovementComponent.GroundFriction` (`self.OriginalGroundFriction`) _charactermovement :!label _label)
          (bind _character_2 (`self.FGet Player Info`))
          (`/Game/AbilitySystem/Core/Blueprints/Characters/Bp_CharacterBase.EvSetCollisionToPawn` _character_2 "ECR_Block")
          (`self.K2_EndAbility`))
        (:`OnBlendOut`
          (goto _label))
        (:`OnInterrupted`
          (goto _label))
        (:`OnCancelled`
          (goto _label))))
    (:`CastFailed`
      (`self.K2_EndAbility`))))