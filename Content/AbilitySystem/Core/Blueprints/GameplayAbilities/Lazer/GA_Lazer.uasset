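; GA_Lazer is a gameplay ability that fires a laser attached to the character's mesh socket.
; On activation it commits, shows the UI cooldown, plays a casting montage, then after a short delay spawns BP_Lazer and enables camera-controlled rotation.
; Skill.lazer.dealDamage events supply targets to damage and push away from the beam's end point with a brief stun.
; Ending removes the draining-cost effect, destroys the laser and restores rotation.
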(event `self.K2_ActivateAbility`
  (`self.K2_CommitAbility`)
  (`self.FDoUICooldown`)
  (`AbilityTask_PlayMontageAndWait.CreatePlayMontageAndWaitProxy` "None" "/Game/AbilitySystem/Animations/Shinbi/AM_Lazer_Casting.AM_Lazer_Casting"
    (:`then`
      (`KismetSystemLibrary.Delay` 0.45)
      (bind _character (`self.FGet Player Info`))
      (bind (_asynctaskproxy _spawnedactor) (`AbilityTask_SpawnActor.SpawnActor` (struct) "/Game/AbilitySystem/Core/Blueprints/GameplayAbilities/Lazer/BP_Lazer.BP_Lazer_C" _character)
        (:`then`
          (bind _output_get (set `self.bp_LazerActor` _spawnedactor))
          (`Actor.K2_AttachToComponent` _output_get (`Character.Mesh` _character) "Lazer" "SnapToTarget" "SnapToTarget" "KeepRelative" true)
          (`/Game/AbilitySystem/Core/Blueprints/Characters/Bp_CharacterBase.EvMakeCameraControlAndRotation` _character true)
          (bind (_asynctaskproxy_2 _payload) (`AbilityTask_WaitGameplayEvent.WaitGameplayEvent` (struct :`TagName` "skill.lazer.dealDamage") null)
            (:`EventReceived`
              (bind (_eventtag _instigator _target _optionalobject _optionalobject2 _contexthandle _instigatortags _targettags _eventmagnitude _targetdata) (break `GameplayEventData` _payload))
              (`self.BP_ApplyGameplayEffectToTarget` _targetdata "/Game/AbilitySystem/Core/Blueprints/GameplayAbilities/Lazer/Attr/GE_Lazer_Damage.GE_Lazer_Damage_C")
              (for _array_element (`AbilitySystemBlueprintLibrary.GetActorsFromTargetData` _targetdata)
                (bind _asbp_character_base (cast `/Game/AbilitySystem/Core/Blueprints/Characters/Bp_CharacterBase` _array_element))
                (`/Game/AbilitySystem/Core/Blueprints/Characters/Bp_CharacterBase.EvPushCharacter` _asbp_character_base (`KismetMathLibrary.Normal` (- (`Actor.K2_GetActorLocation` _asbp_character_base) (`SceneComponent.K2_GetComponentLocation` (`/Game/AbilitySystem/Core/Blueprints/GameplayAbilities/Lazer/BP_Lazer.LazerEndDetection` (cast `/Game/AbilitySystem/Core/Blueprints/GameplayAbilities/Lazer/BP_Lazer` (`self.bp_LazerActor`) :!pure true))))) 500.0 0.3)))))))))

(event `self.K2_OnEndAbility`
  (params (bWasCancelled :type Boolean))
  (`self.BP_RemoveGameplayEffectFromOwnerWithAssetTags` (struct :`GameplayTags` (struct :`(TagName` "skill.lazer.drainingCost"))))
  (`Actor.K2_DestroyActor` (`self.bp_LazerActor`))
  (bind _character (`self.FGet Player Info`))
  (`/Game/AbilitySystem/Core/Blueprints/Characters/Bp_CharacterBase.EvMakeCameraControlAndRotation` _character false))