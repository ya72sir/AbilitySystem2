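; BP_Lazer is a laser beam actor for an ability that periodically signals damage on hostile characters touching its end detection component.
; Overlaps maintain a list of characters hostile to the instigator.
; A looping timer sends that list to the instigator as target data in a Skill.lazer.dealDamage gameplay event.
; Construction and Tick stretch the skeletal beam to the detection component by offsetting BP_AnimLazer's end bone from the original length.
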(event `Ev_SetLocationEndLazer`
  (set `self.BeamOriginalLength` (`KismetMathLibrary.VSize` (- (`SceneComponent.GetSocketLocation` (`self.SkeletalMesh`) "end") (`self.K2_GetActorLocation`)))))

(event `self.ReceiveTick`
  (params (DeltaSeconds :type "Float (single-precision)"))
  (`self.EvEndAnimLazer`))

(event `self.ReceiveBeginPlay`
  (`self.Ev_SetLocationEndLazer`)
  (`KismetSystemLibrary.K2_SetTimerDelegate` (delegate `EvSendDealDamage`) 0.3 true))

(event `EvSendDealDamage`
  (if (`KismetMathLibrary.Conv_IntToBool` (`KismetArrayLibrary.Array_Length` (`self.arrOverlapingCharacters`)))
    (`AbilitySystemBlueprintLibrary.SendGameplayEventToActor` (`self.GetInstigator`) (struct :`TagName` "skill.lazer.dealDamage") (make `GameplayEventData` (struct) null null null null (struct) (struct) (struct) 0.0 (`AbilitySystemBlueprintLibrary.AbilityTargetDataFromActorArray` (`self.arrOverlapingCharacters`))))))

(event `EvEndAnimLazer`
  (bind _asbp_anim_lazer (cast `/Game/AbilitySystem/Core/Assets/Lazer/BP_AnimLazer` (`SkeletalMeshComponent.GetAnimInstance` (`self.SkeletalMesh`))))
  (set `/Game/AbilitySystem/Core/Assets/Lazer/BP_AnimLazer.EndBoneOffset` (`KismetMathLibrary.MakeVector` (- (`KismetMathLibrary.VSize` (- (`SceneComponent.K2_GetComponentLocation` (`self.LazerEndDetection`)) (`self.K2_GetActorLocation`))) (`self.BeamOriginalLength`))) _asbp_anim_lazer))

(event `self.LazerEndDetection.OnComponentBeginOverlap`
  (params (OverlappedComponent :type "PrimitiveComponent Object Reference") (OtherActor :type "Actor Object Reference") (OtherComp :type "PrimitiveComponent Object Reference") (OtherBodyIndex :type Integer) (bFromSweep :type Boolean) (SweepResult :type "HitResult Structure (by ref)"))
  (bind _asbp_character_base (cast `/Game/AbilitySystem/Core/Blueprints/Characters/Bp_CharacterBase` OtherActor))
  (bind _asbp_character_base_2 (cast `/Game/AbilitySystem/Core/Blueprints/Characters/Bp_CharacterBase` (`self.GetInstigator`)))
  (bind _returnvalue (`CppCharacterBase.FCppIsOtherHosttile` _asbp_character_base_2 _asbp_character_base))
  (if _returnvalue
    (`KismetArrayLibrary.Array_AddUnique` (`self.arrOverlapingCharacters`) _asbp_character_base)))

(event `self.LazerEndDetection.OnComponentEndOverlap`
  (params (OverlappedComponent :type "PrimitiveComponent Object Reference") (OtherActor :type "Actor Object Reference") (OtherComp :type "PrimitiveComponent Object Reference") (OtherBodyIndex :type Integer))
  (bind _asbp_character_base (cast `/Game/AbilitySystem/Core/Blueprints/Characters/Bp_CharacterBase` OtherActor))
  (`KismetArrayLibrary.Array_RemoveItem` (`self.arrOverlapingCharacters`) _asbp_character_base))

(fn `UserConstructionScript`
  (`self.Ev_SetLocationEndLazer`)
  (`self.EvEndAnimLazer`))