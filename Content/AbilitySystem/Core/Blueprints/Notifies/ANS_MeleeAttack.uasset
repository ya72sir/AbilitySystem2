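; Anim notify state that opens a melee hit window during attack animations.
; On begin, it casts the mesh owner to Bp_CharacterBase and sets its sword collider to query-only collision.
; On end, it switches that collider back to no collision.
; Both handlers return false when the owner is not a Bp_CharacterBase.
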(fn `Received_NotifyBegin`
  (params (MeshComp :type "SkeletalMeshComponent Object Reference") (Animation :type "AnimSequenceBase Object Reference") (TotalDuration :type "Float (double-precision)"))
  (returns (ReturnValue :type Boolean))
  (bind _asbp_character_base (cast `/Game/AbilitySystem/Core/Blueprints/Characters/Bp_CharacterBase` (`ActorComponent.GetOwner` MeshComp))
    (:`then`
      (`PrimitiveComponent.SetCollisionEnabled` (`/Game/AbilitySystem/Core/Blueprints/Characters/Bp_CharacterBase.SwordColliedr` _asbp_character_base) "QueryOnly")
      (return true))
    (:`CastFailed`
      (return false))))

(fn `Received_NotifyEnd`
  (params (MeshComp :type "SkeletalMeshComponent Object Reference") (Animation :type "AnimSequenceBase Object Reference"))
  (returns (ReturnValue :type Boolean))
  (bind _asbp_character_base (cast `/Game/AbilitySystem/Core/Blueprints/Characters/Bp_CharacterBase` (`ActorComponent.GetOwner` MeshComp))
    (:`then`
      (`PrimitiveComponent.SetCollisionEnabled` (`/Game/AbilitySystem/Core/Blueprints/Characters/Bp_CharacterBase.SwordColliedr` _asbp_character_base) "NoCollision")
      (return true))
    (:`CastFailed`
      (return false))))