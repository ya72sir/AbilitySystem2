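; Base player controller that drives a BPCharacterBase pawn and creates the player's primary HUD.
; On BeginPlay it caches the controlled pawn as the character, then adds the WBP_PrimaryUI widget to the viewport only if that cast succeeds or independently in sequence.
; Axis input moves the pawn relative to camera rotation and turns the view, while Jump and PrimaryAttack presses call the character's jump and melee attack.
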(event `self.ReceiveBeginPlay`
  (`|ExecutionSequence`
    (:`then_0`
      (bind _asbp_character_base (cast `/Game/AbilitySystem/Core/Blueprints/Player/BpCharacterBase` (`self.K2_GetPawn`)))
      (set `self.BPCharacterBase` _asbp_character_base))
    (:`then_1`
      (bind _returnvalue (`|CreateWidget` "/Game/AbilitySystem/Core/UI/WBP_PrimaryUI.WBP_PrimaryUI_C"))
      (bind _output_get (set `self.WBP_PrimaryUI` _returnvalue))
      (`UserWidget.AddToViewport` _output_get 0))))

(event `InputAxis|MoveForward`
  (params (AxisValue :type "Float (single-precision)"))
  (`Pawn.AddMovementInput` (`self.K2_GetPawn`) (`KismetMathLibrary.GetForwardVector` (`PlayerCameraManager.GetCameraRotation` (`self.PlayerCameraManager`))) AxisValue false))

(event `InputAxis|MoveRight`
  (params (AxisValue :type "Float (single-precision)"))
  (`Pawn.AddMovementInput` (`self.K2_GetPawn`) (`KismetMathLibrary.GetRightVector` (`PlayerCameraManager.GetCameraRotation` (`self.PlayerCameraManager`))) AxisValue false))

(event `InputAction|Jump`
  (params (Key :type "Key Structure"))
  (:`Pressed`
    (`Character.Jump` (`self.BPCharacterBase`))))

(event `InputAxis|LookingUp`
  (params (AxisValue :type "Float (single-precision)"))
  (`self.AddPitchInput` AxisValue))

(event `InputAxis|LookingRight`
  (params (AxisValue :type "Float (single-precision)"))
  (`self.AddYawInput` AxisValue))

(event `InputAction|PrimaryAttack`
  (params (Key :type "Key Structure"))
  (:`Pressed`
    (`/Game/AbilitySystem/Core/Blueprints/Player/BpCharacterBase.EvMeleeAttack` (`self.BPCharacterBase`))))

(fn `UserConstructionScript`)