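; Player character Blueprint in the AbilitySystem core that passes health changes on to the player's UI.
; The OnHelathChanged event, grouped in the EvCpp graph, casts the controller to BPPlayerControllerBase and sends the percentage to the health widget inside its primary UI.
; The default event nodes are disabled and the construction script only calls its parent.
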(event `self.BP_OnHelathChanged`
  (params (Health :type "Float (single-precision)") (MaxHealth :type "Float (single-precision)") (percentage :type "Float (single-precision)"))
  (bind _asbpplayer_controller_base (cast `/Game/AbilitySystem/Core/Blueprints/Player/BPPlayerControllerBase` (`self.GetController`)))
  (`/Game/AbilitySystem/Core/UI/WBP_GlassBall.EvSetPercentage` (`/Game/AbilitySystem/Core/UI/WBP_PrimaryUI.WBP_Health` (`/Game/AbilitySystem/Core/Blueprints/Player/BPPlayerControllerBase.WBP_PrimaryUI` _asbpplayer_controller_base)) percentage))

(fn `UserConstructionScript`
  (`parent.UserConstructionScript`))