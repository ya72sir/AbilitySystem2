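; Base player character Blueprint that grants and triggers a Gameplay Ability System melee attack.
; BeginPlay acquires GA_Melee, and a melee attack event tries to activate it by class.
; When the sword collider begins overlapping an actor whose class is exactly BP_EnemyBase, it sends a deal-damage gameplay event to itself with that enemy as target, leaving the damage to the ability system.
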(event `self.ReceiveBeginPlay`
  (`parent.ReceiveBeginPlay`)
  (`self.AquireAbility` "/Game/AbilitySystem/Core/Blueprints/GameplayAbilities/Melee/GA_Melee.GA_Melee_C"))

(event `EvMeleeAttack`
  (`AbilitySystemComponent.TryActivateAbilityByClass` (`self.AbilitySystemComp`) "/Game/AbilitySystem/Core/Blueprints/GameplayAbilities/Melee/GA_Melee.GA_Melee_C" true))

(event `self.ReceiveTick`
  (params (DeltaSeconds :type "Float (single-precision)")))

(event `self.SwordColliedr.OnComponentBeginOverlap`
  (params (OverlappedComponent :type "PrimitiveComponent Object Reference") (OtherActor :type "Actor Object Reference") (OtherComp :type "PrimitiveComponent Object Reference") (OtherBodyIndex :type Integer) (bFromSweep :type Boolean) (SweepResult :type "HitResult Structure (by ref)"))
  (if (!= self OtherActor)
    (if (== (`GameplayStatics.GetObjectClass` OtherActor) "/Game/AbilitySystem/Core/Blueprints/Enemys/BP_EnemyBase.BP_EnemyBase_C")
      (`AbilitySystemBlueprintLibrary.SendGameplayEventToActor` self (struct :`TagName` "skill.melee.dealDamage") (make `GameplayEventData` (struct) null OtherActor)))))

(fn `UserConstructionScript`)