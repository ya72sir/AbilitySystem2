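; Base Gameplay Ability Blueprint that provides shared helpers for abilities owned by Bp_CharacterBase characters.
; EvPushCharacter casts the target actor and forwards a push directed away from the ability's owner, with strength and stun duration, to that character's own push event.
; GetPlayerInfo returns the owning character and its player controller, tolerating a failed controller cast.
; Activate and end events are disabled placeholders.
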(event `EvPushCharacter`
  (params (actor :type "Actor Object Reference") (PushStrength :type "Float (double-precision)") (StunDuration :type "Float (double-precision)"))
  (bind _asbp_character_base (cast `/Game/AbilitySystem/Core/Blueprints/BaseClass/Bp_CharacterBase` actor))
  (`/Game/AbilitySystem/Core/Blueprints/BaseClass/Bp_CharacterBase.EvPushCharacter` _asbp_character_base (`KismetMathLibrary.Normal` (- (`Actor.K2_GetActorLocation` _asbp_character_base) (`Actor.K2_GetActorLocation` (`self.GetOwningActorFromActorInfo`)))) PushStrength StunDuration))

(fn `Get Player Info`
  (returns (Character :type "/Game/AbilitySystem/Core/Blueprints/BaseClass/Bp_CharacterBase Object Reference") (Controller :type "/Game/AbilitySystem/Core/Blueprints/Player/BP_PlayerControllerBase Object Reference"))
  (bind _asbp_character_base (cast `/Game/AbilitySystem/Core/Blueprints/BaseClass/Bp_CharacterBase` (`self.GetOwningActorFromActorInfo`)))
  (bind _asbp_player_controller_base (cast `/Game/AbilitySystem/Core/Blueprints/Player/BP_PlayerControllerBase` (`Pawn.GetController` _asbp_character_base))
    (:`then`
      _)
    (:`CastFailed`
      _))
  (return _asbp_character_base _asbp_player_controller_base))