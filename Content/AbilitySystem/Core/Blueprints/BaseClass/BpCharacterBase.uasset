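; Base character Blueprint that gives characters a Gameplay Ability System melee attack and handles their death.
; It acquires GA_Melee on BeginPlay, and EvMeleeAttack activates it through the ability system component.
; Sword collider overlaps with other characters run a hostility check, then send a damage gameplay event to itself with the victim as target, leaving damage outside this Blueprint.
; Die plays a death montage, waits out its length, then destroys the actor.
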(event `self.ReceiveBeginPlay`
  (`parent.ReceiveBeginPlay`)
  (`self.AquireAbility` "/Game/AbilitySystem/Core/Blueprints/GameplayAbilities/Melee/GA_Melee.GA_Melee_C"))

(event `EvMeleeAttack`
  (`AbilitySystemComponent.TryActivateAbilityByClass` (`self.AbilitySystemComp`) "/Game/AbilitySystem/Core/Blueprints/GameplayAbilities/Melee/GA_Melee.GA_Melee_C" true))

(event `self.ReceiveTick`
  (params (DeltaSeconds :type "Float (single-precision)")))

(event `self.SwordColliedr.OnComponentBeginOverlap`
  (params (OverlappedComponent :type "PrimitiveComponent Object Reference") (OtherActor :type "Actor Object Reference") (OtherComp :type "PrimitiveComponent Object Reference") (OtherBodyIndex :type Integer) (bFromSweep :type Boolean) (SweepResult :type "HitResult Structure (by ref)"))
  (if (!= self OtherActor)
    (bind _asbp_character_base (cast `/Game/AbilitySystem/Core/Blueprints/BaseClass/BpCharacterBase` OtherActor))
    (bind _returnvalue (`self.FCppIsOtherHosttile` _asbp_character_base self))
    (if _returnvalue
      (`AbilitySystemBlueprintLibrary.SendGameplayEventToActor` self (struct :`TagName` "skill.melee.dealDamage") (make `GameplayEventData` (struct) null OtherActor)))))

(event `self.BP_Die`
  (bind _returnvalue (`self.PlayAnimMontage` "/Game/AbilitySystem/Animations/Shinbi/AM_Death_A_Shinbi.AM_Death_A_Shinbi"))
  (`KismetSystemLibrary.Delay` _returnvalue)
  (`self.K2_DestroyActor`))

(fn `UserConstructionScript`)